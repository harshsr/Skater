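; BP_GrindLedge is a spline-defined ledge actor that serves as a rail for grinding.
; Its construction script tiles query-only spline mesh segments at SectionLength intervals along the spline, though each segment's end tangent is fed a location instead of a tangent.
; Query functions turn a hit location into a snap point, tangent and spline distance, then return positions and tangents by distance for movement along it.
; The actor runs no event logic itself.
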(fn `FindSplineTangentNearHit`
  (params (NearHitLocation :type "Vector Structure"))
  (returns (Tangent :type "Vector Structure"))
  (bind _spline (`self.Spline`))
  (return (`SplineComponent.FindTangentClosestToWorldLocation` _spline (`SplineComponent.FindLocationClosestToWorldLocation` _spline NearHitLocation "World") "World")))

(fn `FindSplineTangentNearHitLocation`
  (params (NearHitLocation :type "Vector Structure"))
  (returns (ReturnValue :type "Vector Structure"))
  (bind _spline (`self.Spline`))
  (return (`SplineComponent.FindTangentClosestToWorldLocation` _spline (`SplineComponent.FindLocationClosestToWorldLocation` _spline NearHitLocation "World") "World")))

(fn `GetInitialHitDistanceAlongSpline`
  (params (HitLocaion :type "Vector Structure"))
  (returns (ReturnValue :type "Float (single-precision)"))
  (bind _spline (`self.Spline`))
  (return (`SplineComponent.GetDistanceAlongSplineAtSplineInputKey` _spline (`SplineComponent.FindInputKeyClosestToWorldLocation` _spline HitLocaion))))

(fn `GetInitialSnapPoint`
  (params (HitLocation :type "Vector Structure"))
  (returns (ReturnValue :type "Vector Structure"))
  (return (`SplineComponent.FindLocationClosestToWorldLocation` (`self.Spline`) HitLocation "World")))

(fn `GetNextMovePointAndTangent`
  (params (DistanceOnSpline :type "Float (double-precision)"))
  (returns (NextSnapLocation :type "Vector Structure") (SnapPointTangent :type "Vector Structure"))
  (bind _spline (`self.Spline`))
  (return (`SplineComponent.GetLocationAtDistanceAlongSpline` _spline DistanceOnSpline "World") (`SplineComponent.GetTangentAtDistanceAlongSpline` _spline DistanceOnSpline "World")))

(fn `GetSnapPointAtDistanceAlongSpline`
  (params (DistanceAlongSpline :type "Float (single-precision)"))
  (returns (ReturnValue :type "Vector Structure"))
  (return (`SplineComponent.GetLocationAtDistanceAlongSpline` (`self.Spline`) DistanceAlongSpline "World")))

(fn `GetSplineInformationInitial`
  (params (HitLocation :type "Vector Structure"))
  (returns (SnapToPoint :type "Vector Structure") (SplineDistanceTotal :type "Float (double-precision)") (SnapPointDistance :type "Float (double-precision)"))
  (bind _spline (`self.Spline`))
  (return (`SplineComponent.FindLocationClosestToWorldLocation` _spline HitLocation "World") (`SplineComponent.GetSplineLength` _spline) (`SplineComponent.GetDistanceAlongSplineAtSplineInputKey` _spline (`SplineComponent.FindInputKeyClosestToWorldLocation` _spline HitLocation))))

(fn `GetSplineLength`
  (returns (ReturnValue :type "Float (single-precision)"))
  (return (`SplineComponent.GetSplineLength` (`self.Spline`))))

(fn `GetTangentAtDistanceAlongSpline`
  (params (DistanceAlongSpline :type "Float (single-precision)"))
  (returns (ReturnValue :type "Vector Structure"))
  (return (`SplineComponent.GetTangentAtDistanceAlongSpline` (`self.Spline`) DistanceAlongSpline "World")))

(fn `UserConstructionScript`
  (bind _spline (`self.Spline`))
  (bind _sectionlength (`self.SectionLength`))
  (for _index (range (+ (`KismetMathLibrary.FTrunc` (/ (`SplineComponent.GetSplineLength` (`self.Spline`)) (`self.SectionLength`))) 1))
    (bind _returnvalue (`AddComponent|NODE_AddSplineMeshComponent-0`))
    (`SplineMeshComponent.SetForwardAxis` _returnvalue "Y" true)
    (bind _returnvalue_2 (* _index _sectionlength))
    (bind _returnvalue_3 (* (+ _index 1) _sectionlength))
    (`SplineMeshComponent.SetStartAndEnd` _returnvalue (`SplineComponent.GetLocationAtDistanceAlongSpline` _spline _returnvalue_2 "Local") (`SplineComponent.GetTangentAtDistanceAlongSpline` _spline _returnvalue_2 "Local") (`SplineComponent.GetLocationAtDistanceAlongSpline` _spline _returnvalue_3 "Local") (`SplineComponent.GetLocationAtDistanceAlongSpline` _spline _returnvalue_3 "Local") true)
    (`PrimitiveComponent.SetCollisionEnabled` _returnvalue "QueryOnly")))