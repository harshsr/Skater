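; Physics-sphere roller that drives the player's skateboarding movement, paired with PAWN_SkateTracker, which supplies direction vectors and plays animations.
; In Skate mode, pump, lean and ollie apply forces while Tick clamps speed, adds ground stick and traces along velocity for aligned grind splines.
; Grind mode disables physics and teleports along the spline at entry speed.
; Fanned traces report ground; stepped ballistic traces predict landings to orient the pawn.
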(event `self.ReceiveTick`
  (params (DeltaSeconds :type "Float (single-precision)"))
  (`self.CheckGrinding`)
  (switch `/Game/PrototypeA/Core/V3/E_CurrentMovementMode` (`self.CurrentMovementMode`)
    (:`NewEnumerator0`
      (bind _returnvalue (`PrimitiveComponent.GetPhysicsLinearVelocity` (`self.Sphere`) "None"))
      (`KismetSystemLibrary.PrintString` (`KismetStringLibrary.Conv_DoubleToString` (`KismetMathLibrary.VSize` _returnvalue)) true true (struct :`R` 1.0 :`A` 1.0) DeltaSeconds)
      (`self.ClampVelocity`)
      (`self.StickToGround`)
      (if (not (`self.bGrindCooldownComplete`))
        (bind _output_get (set `self.CurrentGrindCooldown` (+ (`self.CurrentGrindCooldown`) (`GameplayStatics.GetWorldDeltaSeconds`))))
        (if (> _output_get (`self.GrindCooldownTarget`))
          (set `self.bGrindCooldownComplete` true)
          (set `self.CurrentGrindCooldown` 0.0)))
      (if (`self.bOlliNextFrame`)
        (`self.Olli`)))
    (:`NewEnumerator1`
      (`self.Grind`))))

(event `self.FlippingCamera`
  (bind _sphere (`self.Sphere`))
  (bind (_forwardvector _rightvector _upvector _groundtracehitnormal) (message `/Game/PrototypeA/Core/V3/IF_RollerSkate.GetPawnVectors` (`GameplayStatics.GetPlayerPawn` 0)))
  (bind _returnvalue (`PrimitiveComponent.GetPhysicsLinearVelocity` _sphere "None"))
  (bind _returnvalue_2 (`KismetMathLibrary.Cross_VectorVector` (`KismetMathLibrary.Normal` (`KismetMathLibrary.Cross_VectorVector` _groundtracehitnormal (0.0 0.0 1.0))) (0.0 0.0 1.0)))
  (`PrimitiveComponent.SetPhysicsLinearVelocity` _sphere (- _returnvalue (* (`KismetMathLibrary.Normal` _returnvalue_2) (/ (`KismetMathLibrary.Dot_VectorVector` _returnvalue _returnvalue_2) (`KismetMathLibrary.VSize` _returnvalue_2)))) false "None"))

(event `self.AdjustVelocityOnLandedInBoardDirection`
  (params (BoardForwardVector :type "Vector Structure"))
  (bind _sphere (`self.Sphere`))
  (bind _returnvalue (`PrimitiveComponent.GetPhysicsLinearVelocity` _sphere "None"))
  (`PrimitiveComponent.SetPhysicsLinearVelocity` _sphere (* (`KismetMathLibrary.MakeVector` BoardForwardVector_X BoardForwardVector_Y) (`KismetMathLibrary.VSize` (`KismetMathLibrary.MakeVector` (.x _returnvalue) (.y _returnvalue)))) false "None"))

(event `self.AirTrajectoryPrediction`
  (`self.TrajectoryPrediction`))

(event `self.ReceiveBeginPlay`)

(event `self.Pump`
  (params (bAtRest :type Boolean))
  ;[1 1 1] Pump
  (switch `/Game/PrototypeA/Core/V3/E_CurrentMovementMode` (`self.CurrentMovementMode`)
    (:`NewEnumerator0`
      (if bAtRest
        _
        (else
          _))
      (bind _forwardvector (message `/Game/PrototypeA/Core/V3/IF_RollerSkate.GetPawnVectors` (`GameplayStatics.GetPlayerPawn` 0)))
      (bind _output_get (set `self.PumpDirection` _forwardvector))
      (`SkeletalMeshComponent.PlayAnimation` (`/Game/PrototypeA/Core/V3/PAWN_SkateTracker.Max` (cast `/Game/PrototypeA/Core/V3/PAWN_SkateTracker` (`GameplayStatics.GetPlayerPawn` 0) :!pure true)) "/Game/PrototypeA/Assets/Rider/Anim/A_Pump.A_Pump" false)
      (bind (_direction _forcerate) (`Timeline|PumpTimeline` :!via `PlayFromStart`)
        (:`Update`
          (`PrimitiveComponent.AddForce` (`self.Sphere`) (* _output_get (* _forcerate (`self.PumpForce`))) "None" true))))))

(event `self.BodyLean`
  (params (AxisValue :type "Float (double-precision)") (bAtRest :type Boolean))
  (bind _sphere (`self.Sphere`))
  ;[1 1 1] Body Lean
  (if (not bAtRest)
    (switch `/Game/PrototypeA/Core/V3/E_CurrentMovementMode` (`self.CurrentMovementMode`)
      (:`NewEnumerator0`
        (bind _returnvalue (`PrimitiveComponent.GetPhysicsLinearVelocity` _sphere "None"))
        (`PrimitiveComponent.AddForce` _sphere (* (`KismetMathLibrary.Cross_VectorVector` (0.0 0.0 1.0) (`KismetMathLibrary.Normal` _returnvalue)) (* (* (`KismetMathLibrary.FClamp` (/ (`KismetMathLibrary.VSize` _returnvalue) (`self.MaxVelocity`)) 0.05 2.0) 1.0) (* AxisValue (`self.BodyLeanForce`)))) "None" true)))))

(event `self.Olli`
  (bind _aspawn_skate_tracker (cast `/Game/PrototypeA/Core/V3/PAWN_SkateTracker` (`GameplayStatics.GetPlayerPawn` 0) :!pure true))
  (switch `/Game/PrototypeA/Core/V3/E_CurrentMovementMode` (`self.CurrentMovementMode`)
    (:`NewEnumerator0`
      (bind (_forwardvector _rightvector _upvector) (message `/Game/PrototypeA/Core/V3/IF_RollerSkate.GetPawnVectors` (`GameplayStatics.GetPlayerPawn` 0)))
      (`PrimitiveComponent.AddImpulse` (`self.Sphere`) (* (+ (* _forwardvector 0.025) _upvector) (`self.OlliImpulse`)) "None" true)
      (set `self.bOlliNextFrame` false)
      (`SkeletalMeshComponent.PlayAnimation` (`/Game/PrototypeA/Core/V3/PAWN_SkateTracker.Board` _aspawn_skate_tracker) "/Game/PrototypeA/Assets/SkateBoard/Anim/A_Ollie.A_Ollie" false)
      (`SkeletalMeshComponent.PlayAnimation` (`/Game/PrototypeA/Core/V3/PAWN_SkateTracker.Max` _aspawn_skate_tracker) "/Game/PrototypeA/Assets/Rider/Anim/A_OllieJump.A_OllieJump" false))
    (:`NewEnumerator1`
      (`self.ChangeMovementMode` "NewEnumerator0")
      (set `self.bOlliNextFrame` true)
      (set `self.bGrindCooldownComplete` false))))

(fn `ChangeMovementMode`
  (params (NewMovementMode :type "/Game/PrototypeA/Core/V3/E_CurrentMovementMode Enum" :default "NewEnumerator0"))
  (bind _sphere (`self.Sphere`))
  (bind _aspawn_skate_tracker (cast `/Game/PrototypeA/Core/V3/PAWN_SkateTracker` (`GameplayStatics.GetPlayerPawn` 0) :!pure true))
  (bind _output_get (set `self.CurrentMovementMode` NewMovementMode))
  (switch `/Game/PrototypeA/Core/V3/E_CurrentMovementMode` _output_get
    (:`NewEnumerator0`
      (`PrimitiveComponent.SetSimulatePhysics` _sphere true)
      (bind _forwardvector (message `/Game/PrototypeA/Core/V3/IF_RollerSkate.GetPawnVectors` (`GameplayStatics.GetPlayerPawn` 0)))
      (`PrimitiveComponent.SetPhysicsLinearVelocity` _sphere (* _forwardvector (`KismetMathLibrary.VSize` (`self.VelocityOnGrindStart`))) false "None")
      (`SkeletalMeshComponent.PlayAnimation` (`/Game/PrototypeA/Core/V3/PAWN_SkateTracker.Max` _aspawn_skate_tracker) "/Game/PrototypeA/Assets/Rider/Anim/A_Skate.A_Skate" true)
      (`SkeletalMeshComponent.PlayAnimation` (`/Game/PrototypeA/Core/V3/PAWN_SkateTracker.Board` _aspawn_skate_tracker) "/Game/PrototypeA/Assets/SkateBoard/Anim/A_Stable.A_Stable" true))
    (:`NewEnumerator1`
      (bind _returnvalue (`PrimitiveComponent.GetPhysicsLinearVelocity` (`self.Sphere`) "None"))
      (set `self.VelocityOnGrindStart` _returnvalue)
      (`PrimitiveComponent.SetSimulatePhysics` (`self.Sphere`) false))))

(fn `CheckGrinding`
  (bind _returnvalue (`self.K2_GetActorLocation`))
  (switch `/Game/PrototypeA/Core/V3/E_CurrentMovementMode` (`self.CurrentMovementMode`)
    (:`NewEnumerator0`
      (if (`self.bGrindCooldownComplete`)
        (bind _returnvalue_2 (`PrimitiveComponent.GetPhysicsLinearVelocity` (`self.Sphere`) "None"))
        (bind _outhit (`KismetSystemLibrary.LineTraceSingle` :`Start` _returnvalue :`End` (+ _returnvalue (* _returnvalue_2 1)) :`TraceChannel` "TraceTypeQuery3" :`TraceColor` (struct :`R` 0.000555 :`B` 1.0 :`A` 1.0)))
        (if (`GameplayStatics.BreakHitResult` _outhit)
          (if (< (`.Distance` (`GameplayStatics.BreakHitResult` _outhit)) 50.0)
            (bind _tangent (message `/Game/PrototypeA/Core/Grinding/IF_Grind.FindSplineTangentNearHit` (`.HitActor` (`GameplayStatics.BreakHitResult` _outhit)) (`.ImpactPoint` (`GameplayStatics.BreakHitResult` _outhit))))
            (bind _returnvalue_3 (`PrimitiveComponent.GetPhysicsLinearVelocity` (`self.Sphere`) "None"))
            (if (> (`KismetMathLibrary.VSize` _returnvalue_3) 250.0)
              (bind _returnvalue_4 (`KismetMathLibrary.Dot_VectorVector` (`KismetMathLibrary.Normal` _tangent) (`KismetMathLibrary.Normal` _returnvalue_3)))
              (if (> (`KismetMathLibrary.Abs` _returnvalue_4) 0.9)
                (`KismetSystemLibrary.PrintString` "Grind!!" true true (struct :`R` 1.0 :`G` 0.951255 :`A` 1.0))
                (set `self.bMovingInSplineDirection` (> _returnvalue_4 0.0))
                (bind _output_get (set `self.GrindActor` (`.HitActor` (`GameplayStatics.BreakHitResult` _outhit))))
                (bind (_snaptopoint _splinedistancetotal _snappointdistance) (message `/Game/PrototypeA/Core/Grinding/IF_Grind.GetSplineInformationInitial` _output_get (`.ImpactPoint` (`GameplayStatics.BreakHitResult` _outhit))))
                (set `self.SnapPoint` _snaptopoint)
                (set `self.TotalSplineDistance` _splinedistancetotal)
                (set `self.InitialSplineDistance` _snappointdistance)
                (`self.ChangeMovementMode` "NewEnumerator1")
                (set `self.bGrindSnapHappened` false)))))))))

(fn `ClampVelocity`
  (bind _returnvalue (`PrimitiveComponent.GetPhysicsLinearVelocity` (`self.Sphere`) "None"))
  (`PrimitiveComponent.SetPhysicsLinearVelocity` (`self.Sphere`) (* (`KismetMathLibrary.Normal` _returnvalue) (`KismetMathLibrary.FClamp` (`KismetMathLibrary.VSize` _returnvalue) 0.0 (`self.MaxVelocity`))) false "None"))

(fn `GetPawnVectors`
  (returns (ForwardVector :type "Vector Structure") (RightVector :type "Vector Structure") (UpVector :type "Vector Structure") (GroundTraceHitNormal :type "Vector Structure"))
  (return (0.0 0.0 0.0) (0.0 0.0 0.0) (0.0 0.0 0.0) (0.0 0.0 0.0)))

(fn `GetRollerVelocity`
  (returns (Velocity :type "Vector Structure"))
  (bind _returnvalue (`PrimitiveComponent.GetPhysicsLinearVelocity` (`self.Sphere`) "None"))
  (return _returnvalue))

(fn `Grind`
  (bind (_snappoint_x _snappoint_y _snappoint_z) (`KismetMathLibrary.BreakVector` (`self.SnapPoint`)))
  (bind _aspawn_skate_tracker (cast `/Game/PrototypeA/Core/V3/PAWN_SkateTracker` (`GameplayStatics.GetPlayerPawn` 0) :!pure true))
  (bind _returnvalue (+ (* (`KismetMathLibrary.VSize` (`self.VelocityOnGrindStart`)) (`GameplayStatics.GetWorldDeltaSeconds`)) (`self.CurrentGrindDistance`)))
  (bind _returnvalue_2 (- (`self.CurrentGrindDistance`) (* (`KismetMathLibrary.VSize` (`self.VelocityOnGrindStart`)) (`GameplayStatics.GetWorldDeltaSeconds`))))
  (switch `/Game/PrototypeA/Core/V3/E_CurrentMovementMode` (`self.CurrentMovementMode`)
    (:`NewEnumerator1`
      (if (`self.bGrindSnapHappened`)
        (if (`self.bMovingInSplineDirection`)
          (if (> _returnvalue (`self.TotalSplineDistance`))
            (`self.ChangeMovementMode` "NewEnumerator0")
            (else
              (bind (_nextsnaplocation _snappointtangent) (message `/Game/PrototypeA/Core/Grinding/IF_Grind.GetNextMovePointAndTangent` (`self.GrindActor`) _returnvalue))
              (`self.K2_SetActorLocation` (`KismetMathLibrary.MakeVector` (.x _nextsnaplocation) (.y _nextsnaplocation) (+ (.z _nextsnaplocation) (`self.GrindZOffset`))) false true)
              (`SceneComponent.K2_SetWorldRotation` (`/Game/PrototypeA/Core/V3/PAWN_SkateTracker.RotationTracker` (cast `/Game/PrototypeA/Core/V3/PAWN_SkateTracker` (`GameplayStatics.GetPlayerPawn` 0) :!pure true)) (`KismetMathLibrary.MakeRotFromX` _snappointtangent) false true)
              (set `self.CurrentGrindDistance` _returnvalue)))
          (elif (< _returnvalue_2 0.0)
            (`self.ChangeMovementMode` "NewEnumerator0")
            (else
              (bind (_nextsnaplocation_2 _snappointtangent_2) (message `/Game/PrototypeA/Core/Grinding/IF_Grind.GetNextMovePointAndTangent` (`self.GrindActor`) _returnvalue_2))
              (`self.K2_SetActorLocation` (`KismetMathLibrary.MakeVector` (.x _nextsnaplocation_2) (.y _nextsnaplocation_2) (+ (.z _nextsnaplocation_2) (`self.GrindZOffset`))) false true)
              (`SceneComponent.K2_SetWorldRotation` (`/Game/PrototypeA/Core/V3/PAWN_SkateTracker.RotationTracker` (cast `/Game/PrototypeA/Core/V3/PAWN_SkateTracker` (`GameplayStatics.GetPlayerPawn` 0) :!pure true)) (`KismetMathLibrary.MakeRotFromX` (* _snappointtangent_2 -1)) false true)
              (set `self.CurrentGrindDistance` _returnvalue_2))))
        (else
          (`self.K2_SetActorLocation` (`KismetMathLibrary.MakeVector` _snappoint_x _snappoint_y (+ _snappoint_z (`self.GrindZOffset`))) false true)
          (set `self.bGrindSnapHappened` true)
          (set `self.CurrentGrindDistance` (`self.InitialSplineDistance`))
          (`SkeletalMeshComponent.PlayAnimation` (`/Game/PrototypeA/Core/V3/PAWN_SkateTracker.Max` _aspawn_skate_tracker) "/Game/PrototypeA/Assets/Rider/Anim/A_Grind.A_Grind" true)
          (`SkeletalMeshComponent.PlayAnimation` (`/Game/PrototypeA/Core/V3/PAWN_SkateTracker.Board` _aspawn_skate_tracker) "/Game/PrototypeA/Assets/SkateBoard/Anim/A_GrinBoard.A_GrinBoard" true))))))

(fn `ReportGroundCondition`
  (returns (GroundTraceHit :type "HitResult Structure"))
  (locals (LastHit :type "HitResult Structure"))
  (bind _returnvalue (`self.K2_GetActorLocation`))
  (bind _returnvalue_2 (`self.K2_GetActorLocation`))
  (bind _lasthit_bblockinghit (`GameplayStatics.BreakHitResult` (`local.LastHit`)))
  (for (_array_element _array_index) (`self.AngleArrayForGroundChecks`)
    (bind _returnvalue_3 (`KismetMathLibrary.Conv_IntToDouble` _array_element))
    (bind _outhit (`KismetSystemLibrary.LineTraceSingle` :`Start` _returnvalue_2 :`End` (+ _returnvalue_2 (* (+ (* (* (`self.GetActorUpVector`) -1) (`KismetMathLibrary.DegCos` _returnvalue_3)) (* (`KismetMathLibrary.DegSin` _returnvalue_3) (`SceneComponent.GetForwardVector` (`/Game/PrototypeA/Core/V3/PAWN_SkateTracker.Boom` (cast `/Game/PrototypeA/Core/V3/PAWN_SkateTracker` (`GameplayStatics.GetPlayerPawn` 0) :!pure true))))) 65)) :`TraceChannel` "TraceTypeQuery1" :`bTraceComplex` true :`TraceColor` (`KismetMathLibrary.MakeColor` (/ (`KismetMathLibrary.Conv_IntToDouble` _array_index) 5.0))))
    (bind _output_get (set `local.LastHit` _outhit))
    (if (`GameplayStatics.BreakHitResult` _output_get)
      (break)))
  (if _lasthit_bblockinghit
    (return (`local.LastHit`))
    (else
      (for _array_element_2 (`self.AngleArrayForGroundChecks`)
        (bind _returnvalue_4 (`KismetMathLibrary.Conv_IntToDouble` _array_element_2))
        (bind _outhit_2 (`KismetSystemLibrary.LineTraceSingle` _returnvalue (+ _returnvalue (* (+ (* (* (`self.GetActorUpVector`) -1) (`KismetMathLibrary.DegCos` _returnvalue_4)) (* (`KismetMathLibrary.DegSin` _returnvalue_4) (`SceneComponent.GetRightVector` (`/Game/PrototypeA/Core/V3/PAWN_SkateTracker.Boom` (cast `/Game/PrototypeA/Core/V3/PAWN_SkateTracker` (`GameplayStatics.GetPlayerPawn` 0) :!pure true))))) 65)) "TraceTypeQuery1" true))
        (bind _output_get_2 (set `local.LastHit` _outhit_2))
        (if (`GameplayStatics.BreakHitResult` _output_get_2)
          (break)))
      (return (`local.LastHit`)))))

(fn `StickToGround`
  (bind _returnvalue (`GameplayStatics.GetPlayerPawn` 0))
  (switch `/Game/PrototypeA/Core/V3/E_CurrentMovementMode` (`self.CurrentMovementMode`)
    (:`NewEnumerator0`
      (if (`/Game/PrototypeA/Core/V3/PAWN_SkateTracker.bGrounded` (cast `/Game/PrototypeA/Core/V3/PAWN_SkateTracker` _returnvalue :!pure true))
        (bind (_forwardvector _rightvector _upvector) (message `/Game/PrototypeA/Core/V3/IF_RollerSkate.GetPawnVectors` _returnvalue))
        (`PrimitiveComponent.AddForce` (`self.Sphere`) (* _upvector -1000) "None" true)))))

(fn `TrajectoryPrediction`
  (locals (TimeStepArray :type "Array of Float (double-precision)") (InitialVelocity :type "Vector Structure" :default (0.0 0.0 0.0)) (Displacement :type "Vector Structure") (FinalVelocity :type "Vector Structure") (bFoundGround :type Boolean) (Hit :type "HitResult Structure") (HitIndex :type Integer) (ProjectedVelocityDirection :type "Vector Structure"))
  (bind _timesteparray (`local.TimeStepArray`))
  (bind _returnvalue (+ (`self.K2_GetActorLocation`) (`local.Displacement`)))
  (`|ExecutionSequence`
    (:`then_0`
      (for _ (range 101)
        (`KismetArrayLibrary.Array_Add` _timesteparray (+ (`|GetArrayItem` _timesteparray (`KismetArrayLibrary.Array_LastIndex` _timesteparray)) 0.05))))
    (:`then_1`
      (bind _returnvalue_2 (`PrimitiveComponent.GetPhysicsLinearVelocity` (`self.Sphere`) "None"))
      (set `local.InitialVelocity` _returnvalue_2)
      (for (_array_element _array_index) (`local.TimeStepArray`)
        (bind _returnvalue_3 (- _array_element 0.1))
        (set `local.Displacement` (+ (* (`local.InitialVelocity`) _returnvalue_3) (* (* (* _returnvalue_3 _returnvalue_3) 0.5) (0.0 0.0 -980.0))))
        (bind _output_get (set `local.FinalVelocity` (+ (`local.InitialVelocity`) (* _returnvalue_3 (0.0 0.0 -980.0)))))
        (bind _outhit (`KismetSystemLibrary.LineTraceSingle` :`Start` _returnvalue :`End` (+ _returnvalue (* (`KismetMathLibrary.Normal` _output_get) (+ (* (`KismetMathLibrary.VSize` _output_get) 0.05) (* (* (* 0.05 0.05) 0.5) 980.0)))) :`TraceChannel` "TraceTypeQuery1" :`DrawDebugType` "ForDuration" :`TraceColor` (struct :`R` 0.951328 :`B` 1.0 :`A` 1.0) :`TraceHitColor` (struct :`G` 0.854231 :`B` 1.0 :`A` 1.0)))
        (bind _output_get_2 (set `local.Hit` _outhit))
        (bind (_bblockinghit _binitialoverlap _time _distance _location _impactpoint _normal) (`GameplayStatics.BreakHitResult` _output_get_2))
        (if _bblockinghit
          (set `local.ProjectedVelocityDirection` (`KismetMathLibrary.Normal` (`KismetMathLibrary.ProjectVectorOnToPlane` (`local.FinalVelocity`) _normal)))
          (set `local.HitIndex` _array_index)
          (break)))
      (message `/Game/PrototypeA/Core/V3/IF_RollerSkate.OrientToLanding` (`GameplayStatics.GetPlayerPawn` 0) (`local.Hit`) (* (`local.HitIndex`) 0.05) false (`local.ProjectedVelocityDirection`)))))

(fn `UserConstructionScript`)