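; BP_SkatePhysics is a prototype skateboarding physics Blueprint that adds the pump push to a physics-driven root sphere.
; In Skate mode, Pump plays the skater's pump animation and captures the RotationTracker's forward direction.
; A timeline curve scaled by PumpForce then applies mass-independent acceleration along that fixed direction.
; Tick prints the sphere's current speed each frame for debugging.
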(event `self.ReceiveTick`
  (params (DeltaSeconds :type "Float (single-precision)"))
  (bind _returnvalue (`PrimitiveComponent.GetPhysicsLinearVelocity` (`self.RootSphere`) "None"))
  (`KismetSystemLibrary.PrintString` (`KismetStringLibrary.Conv_DoubleToString` (`KismetMathLibrary.VSize` _returnvalue)) true true (struct :`R` 1.0 :`G` 0.390478 :`A` 1.0) DeltaSeconds))

(event `self.Pump`
  (switch `ESkateMode` (`self.CurrentSkateMode`)
    (:`Skate`
      (`SkeletalMeshComponent.PlayAnimation` (`Skater.MaxMesh` (`self.SkaterRef`)) "/Game/PrototypeA/Assets/Rider/Anim/A_Pump.A_Pump" false)
      (bind _output_get (set `self.PumpDirection` (`SceneComponent.GetForwardVector` (`Skater.RotationTracker` (`self.SkaterRef`)))))
      (bind (_direction _forcerate) (`Timeline|Timeline` :!via `PlayFromStart`)
        (:`Update`
          (`PrimitiveComponent.AddForce` (`self.RootSphere`) (* _output_get (* _forcerate (`self.PumpForce`))) "None" true))))))

(fn `UserConstructionScript`)