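; Skater Blueprint that smooths the camera boom and character mesh rotation, both following a RotationTracker component.
; CameraRotation eases the boom toward the tracker's yaw at a fixed downward pitch with no roll.
; MeshRotation eases MaxMesh toward the tracker's full rotation, quickly when Grounded and much more slowly in the air.
; Tick and BeginPlay are unused, and nothing in this graph calls the two rotation events or sets TickDelta and Grounded.
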(event `self.CameraRotation`
  (bind _cameraboom (`self.CameraBoom`))
  (bind (_returnvalue_roll _returnvalue_pitch _returnvalue_yaw) (`KismetMathLibrary.BreakRotator` (`SceneComponent.K2_GetComponentRotation` (`self.RotationTracker`))))
  (bind (_returnvalue_roll_2 _returnvalue_pitch_2 _returnvalue_yaw_2) (`KismetMathLibrary.BreakRotator` (`SceneComponent.K2_GetComponentRotation` _cameraboom)))
  (if (`self.bGrounded`)
    _
    (else
      _))
  (`SceneComponent.K2_SetWorldRotation` _cameraboom (`KismetMathLibrary.RInterpTo` (`KismetMathLibrary.MakeRotator` 0.0 _returnvalue_pitch_2 _returnvalue_yaw_2) (`KismetMathLibrary.MakeRotator` 0.0 -15.0 _returnvalue_yaw) (`self.TickDelta`) 10.0) false false))

(event `self.MeshRotation`
  (bind _maxmesh (`self.MaxMesh`))
  (bind _maxmesh_2 (`self.MaxMesh`))
  (bind (_returnvalue_roll _returnvalue_pitch _returnvalue_yaw) (`KismetMathLibrary.BreakRotator` (`SceneComponent.K2_GetComponentRotation` _maxmesh)))
  (bind (_returnvalue_roll_2 _returnvalue_pitch_2 _returnvalue_yaw_2) (`KismetMathLibrary.BreakRotator` (`SceneComponent.K2_GetComponentRotation` (`self.RotationTracker`))))
  (bind (_returnvalue_roll_3 _returnvalue_pitch_3 _returnvalue_yaw_3) (`KismetMathLibrary.BreakRotator` (`SceneComponent.K2_GetComponentRotation` _maxmesh_2)))
  (bind (_returnvalue_roll_4 _returnvalue_pitch_4 _returnvalue_yaw_4) (`KismetMathLibrary.BreakRotator` (`SceneComponent.K2_GetComponentRotation` (`self.RotationTracker`))))
  (bind (_returnvalue_roll_5 _returnvalue_pitch_5 _returnvalue_yaw_5) (`KismetMathLibrary.BreakRotator` (`KismetMathLibrary.RInterpTo` (`KismetMathLibrary.MakeRotator` _returnvalue_roll _returnvalue_pitch _returnvalue_yaw) (`KismetMathLibrary.MakeRotator` _returnvalue_roll_4 _returnvalue_pitch_4 _returnvalue_yaw_4) (`self.TickDelta`) 1.0)))
  (bind (_returnvalue_roll_6 _returnvalue_pitch_6 _returnvalue_yaw_6) (`KismetMathLibrary.BreakRotator` (`KismetMathLibrary.RInterpTo` (`KismetMathLibrary.MakeRotator` _returnvalue_roll_3 _returnvalue_pitch_3 _returnvalue_yaw_3) (`KismetMathLibrary.MakeRotator` _returnvalue_roll_2 _returnvalue_pitch_2 _returnvalue_yaw_2) (`self.TickDelta`) 10.0)))
  (if (`self.bGrounded`)
    (`SceneComponent.K2_SetWorldRotation` _maxmesh_2 (`KismetMathLibrary.MakeRotator` _returnvalue_roll_6 _returnvalue_pitch_6 _returnvalue_yaw_6) false false)
    (else
      (`SceneComponent.K2_SetWorldRotation` _maxmesh (`KismetMathLibrary.MakeRotator` _returnvalue_roll_5 _returnvalue_pitch_5 _returnvalue_yaw_5) false false))))

(fn `UserConstructionScript`)